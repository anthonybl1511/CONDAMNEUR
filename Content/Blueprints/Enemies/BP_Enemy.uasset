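; Base Doom-style enemy character drawn as a Paper2D flipbook sprite and driven by a behavior tree on BP_DoomEnemyAI.
; Tick yaws the sprite toward the player camera as a billboard and picks walk or idle from velocity.
; Damage pauses that switching for the hurt flipbook, while death stops the AI, disables capsule collision and plays dying, then dead.
; MeleeAttack and RangedAttack are empty events here.
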(event `self.ReceiveBeginPlay`
  (bind _asbp_doom_enemy_ai (cast `/Game/Blueprints/Enemies/AI/BP_DoomEnemyAI` (`self.GetController`)))
  (`AIController.RunBehaviorTree` _asbp_doom_enemy_ai (`self.BehaviorTree`)))

(event `self.ReceiveTick`
  (params (DeltaSeconds :type "Float (single-precision)"))
  (`self.SpriteFacePlayer`
    (:`Out`
      (if (not (or (`self.isDead`) (`self.pauseAnim`)))
        (`self.CheckIfWalking`
          (:`Out`
            (`self.SetFlipbook` (`self.WalkingAnim`) (`self.IdleAnim`))))))))

(event `self.TakeDamage`
  (params (CueData :type "GameplayCueParameters Structure"))
  (bind _enemysprite (`self.EnemySprite`))
  (`parent.TakeDamage` CueData)
  (if (not (`self.isDead`))
    (set `self.pauseAnim` true)
    (`PaperFlipbookComponent.SetFlipbook` _enemysprite (`self.DamagedAnim`))
    (`KismetSystemLibrary.Delay` (`PaperFlipbookComponent.GetFlipbookLength` _enemysprite))
    (set `self.pauseAnim` false)))

(event `self.KillCharacter`
  (bind _enemysprite (`self.EnemySprite`))
  (`parent.KillCharacter`)
  (bind _asbp_doom_enemy_ai (cast `/Game/Blueprints/Enemies/AI/BP_DoomEnemyAI` (`self.GetController`)))
  (`BrainComponent.StopLogic` (`AIController.BrainComponent` _asbp_doom_enemy_ai) "")
  (set `self.isDead` true)
  (`PrimitiveComponent.SetCollisionEnabled` (`self.CapsuleComponent`) "NoCollision")
  (`PaperFlipbookComponent.SetFlipbook` _enemysprite (`self.DyingAnim`))
  (`KismetSystemLibrary.Delay` (`PaperFlipbookComponent.GetFlipbookLength` _enemysprite))
  (`PaperFlipbookComponent.SetFlipbook` (`self.EnemySprite`) (`self.DeadAnim`)))

(event `MeleeAttack`)

(event `RangedAttack`)

(fn `SetFlipbook`
  (params (Walking :type "PaperFlipbook Object Reference") (Idle :type "PaperFlipbook Object Reference"))
  (bind _enemysprite (`self.EnemySprite`))
  (if (`self.isWalking`)
    (`PaperFlipbookComponent.SetFlipbook` _enemysprite Walking)
    (else
      (`PaperFlipbookComponent.SetFlipbook` _enemysprite Idle))))

(fn `UserConstructionScript`)