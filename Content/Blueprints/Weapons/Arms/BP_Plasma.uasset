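; BP_Plasma is the player's plasma weapon, drawn as a flipbook sprite in a first-person game.
; InitializeWeapon shows the idle sprite and caches the player's BP_FirstPersonCharacter.
; ShootPlasma triggers a brief point-light muzzle flash, updates the player UI and spawns a BP_PlasmaProjectile at the spawn point.
; It plays the shoot flipbook, using a delay of that flipbook's length before returning to idle.
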(event `/Game/Blueprints/Weapons/BPI_PlayerWeapon.InitializeWeapon`
  ;[1 1 1] Equip pistol
  (`PaperFlipbookComponent.SetFlipbook` (`self.GunSprite`) (`self.idlePlasma`))
  (`SceneComponent.SetHiddenInGame` (`self.GunSprite`) false false)
  (bind _asbp_first_person_character (cast `/Game/FirstPerson/Blueprints/BP_FirstPersonCharacter` (`GameplayStatics.GetPlayerPawn` 0)))
  (set `self.Player` _asbp_first_person_character))

(event `Shoot Plasma`
  (bind _gunsprite (`self.GunSprite`))
  ;[1 1 1] Plasma shoot animation
  (`self.MuzzleFlash`)
  (`/Game/FirstPerson/Blueprints/BP_FirstPersonCharacter.UpdateUI` (`self.Player`))
  (`|SpawnActorFromClass` "/Game/Blueprints/Weapons/Abilities/Plasma/BP_PlasmaProjectile.BP_PlasmaProjectile_C" (`SceneComponent.K2_GetComponentToWorld` (`self.PlasmaSpawnPoint`)) "Undefined" "MultiplyWithRoot" null null)
  (`PaperFlipbookComponent.SetFlipbook` _gunsprite (`self.shootPlasma`))
  (`KismetSystemLibrary.Delay` (`PaperFlipbookComponent.GetFlipbookLength` _gunsprite))
  (`PaperFlipbookComponent.SetFlipbook` (`self.GunSprite`) (`self.idlePlasma`)))

(event `MuzzleFlash`
  (bind _pointlight (`self.PointLight`))
  ;[1 1 1] Muzzle flash
  (`SceneComponent.SetHiddenInGame` _pointlight false false)
  (`KismetSystemLibrary.Delay` 0.25)
  (`SceneComponent.SetHiddenInGame` _pointlight true false))

(fn `UserConstructionScript`
  (`parent.UserConstructionScript`))