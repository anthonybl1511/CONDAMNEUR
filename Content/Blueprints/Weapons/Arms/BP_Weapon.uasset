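; Weapon Blueprint that displays a Paper2D flipbook gun sprite and handles its bob while moving.
; A SceneCaptureComponent2D captures only the gun sprite, whose starting relative location is cached on BeginPlay.
; WeaponBobbing plays the WeaponAnim sequence during movement, otherwise stops it and interpolates the sprite back to that location.
; InitializeWeapon resets the sprite by calling SetFlipbook with no asset and hiding it.
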(event `self.ReceiveBeginPlay`
  (`SceneCaptureComponent.ShowOnlyComponent` (`self.SceneCaptureComponent2D`) (`self.GunSprite`))
  (set `self.WeaponLocation` (`SceneComponent.RelativeLocation` (`self.GunSprite`))))

(event `/Game/Blueprints/Weapons/BPI_PlayerWeapon.InitializeWeapon`
  (bind _gunsprite (`self.GunSprite`))
  (`PaperFlipbookComponent.SetFlipbook` _gunsprite null)
  (`SceneComponent.SetHiddenInGame` _gunsprite true false))

(event `WeaponBobbing`
  (params (isMoving :type Boolean) (DeltaTime :type "Float (double-precision)"))
  (bind _gunsprite (`self.GunSprite`))
  (bind _sequenceplayer (`ActorSequenceComponent.SequencePlayer` (`self.WeaponAnim`)))
  (if isMoving
    (`MovieSceneSequencePlayer.Play` _sequenceplayer)
    (else
      (`MovieSceneSequencePlayer.Stop` _sequenceplayer)
      (`SceneComponent.K2_SetRelativeLocation` _gunsprite (`KismetMathLibrary.VInterpTo` (`SceneComponent.RelativeLocation` _gunsprite) (`self.WeaponLocation`) DeltaTime 10.0) false false))))

(fn `UserConstructionScript`)