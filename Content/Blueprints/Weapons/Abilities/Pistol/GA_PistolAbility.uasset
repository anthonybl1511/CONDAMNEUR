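; Gameplay Ability that fires the player's pistol.
; ShootWeapon checks that an attribute is above zero, applies the bullet-spend effect to the owner and calls Shoot on the pistol.
; It then line-traces on Visibility from the first-person camera out to WeaponRange and calls ApplyEffect on any BP_DefaultFirstPersonCharacter hit.
; Player and pistol references are lazily cached, with the pistol taken from the player's WeaponActor child actor.
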(event `self.ShootWeapon`
  (bind _playerpistolweapon (`self.PlayerPistolWeapon`))
  ;[1 1 1] Shooting
  (`self.GetPlayer`)
  (if (> (`.ReturnValue` (`AbilitySystemBlueprintLibrary.GetFloatAttributeFromAbilitySystemComponent` (`FirstPersonCharacter.AbilitySystemComponent` (`self.Player`)) (struct :`AttributeName` "Bullets" :`Attribute` "/Script/CONDAMNEUR.FirstPersonAttributeSet:Bullets" :`AttributeOwner` "/Script/CoreUObject.Class'\"/Script/CONDAMNEUR.FirstPersonAttributeSet\"'"))) 0.0)
    (`self.GetWeapon`)
    (`/Engine/EditorBlueprintResources/StandardMacros.IsValid` _playerpistolweapon
      (:`Is Valid`
        (`self.BP_ApplyGameplayEffectToOwner` "/Game/Blueprints/Weapons/Abilities/Pistol/GE_PlayerBulletSpend.GE_PlayerBulletSpend_C")
        (`/Game/Blueprints/Weapons/Arms/BP_Pistol.Shoot` _playerpistolweapon)
        (bind _actor (`self.GetLineTrace`))
        (bind _asbp_default_first_person_character (cast `/Game/Blueprints/BP_DefaultFirstPersonCharacter` _actor))
        (`self.ApplyEffect` (`self.Player`) _asbp_default_first_person_character)))))

(fn `GetLineTrace`
  (returns (Actor :type "Actor Object Reference"))
  (bind _firstpersoncamera (`/Game/FirstPerson/Blueprints/BP_FirstPersonCharacter.FirstPersonCamera` (`self.Player`)))
  (bind _returnvalue (`SceneComponent.K2_GetComponentLocation` _firstpersoncamera))
  (bind _outhit (`KismetSystemLibrary.LineTraceSingle` _returnvalue (+ _returnvalue (* (`SceneComponent.GetForwardVector` _firstpersoncamera) (`self.WeaponRange`))) "TraceTypeQuery1"))
  (bind (_bblockinghit _binitialoverlap _time _distance _location _impactpoint _normal _impactnormal _physmat _hitactor) (`GameplayStatics.BreakHitResult` _outhit))
  (`/Engine/EditorBlueprintResources/StandardMacros.IsValid` _hitactor
    (:`Is Valid`
      (return _hitactor))))

(fn `GetPlayer`
  (bind _returnvalue_owneractor (break `GameplayAbilityActorInfo` (`self.GetActorInfo`)))
  (`/Engine/EditorBlueprintResources/StandardMacros.IsValid` (`self.Player`)
    (:`Is Valid`
      _)
    (:`Is Not Valid`
      (bind _asbp_first_person_character (cast `/Game/FirstPerson/Blueprints/BP_FirstPersonCharacter` _returnvalue_owneractor))
      (set `self.Player` _asbp_first_person_character)))
  (return))

(fn `GetWeapon`
  (`/Engine/EditorBlueprintResources/StandardMacros.IsValid` (`self.PlayerPistolWeapon`)
    (:`Is Valid`
      _)
    (:`Is Not Valid`
      (bind _asbp_pistol (cast `/Game/Blueprints/Weapons/Arms/BP_Pistol` (`ChildActorComponent.ChildActor` (`/Game/FirstPerson/Blueprints/BP_FirstPersonCharacter.WeaponActor` (`self.Player`)))))
      (set `self.PlayerPistolWeapon` _asbp_pistol)))
  (return))