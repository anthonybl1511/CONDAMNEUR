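; GA_EnemyBulletAbility is a gameplay ability that gives the rock enemy a hitscan shot against the first-person player character.
; ShootWeapon caches the owning BP_RockEnemy, then line-traces on Visibility from its capsule along the forward vector for WeaponRange.
; If the hit actor is a BP_DefaultFirstPersonCharacter, ApplyEffect runs with the enemy as attacker.
; The trace leaves persistent debug lines.
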(event `self.ShootWeapon`
  (`self.GetEnemy`)
  (bind _actor (`self.GetLineTrace`))
  (bind _asbp_default_first_person_character (cast `/Game/Blueprints/BP_DefaultFirstPersonCharacter` _actor))
  (`self.ApplyEffect` (`self.RockEnemy`) _asbp_default_first_person_character))

(fn `GetEnemy`
  (bind _returnvalue_owneractor (break `GameplayAbilityActorInfo` (`self.GetActorInfo`)))
  (`/Engine/EditorBlueprintResources/StandardMacros.IsValid` (`self.RockEnemy`)
    (:`Is Valid`
      _)
    (:`Is Not Valid`
      (bind _asbp_rock_enemy (cast `/Game/Blueprints/Enemies/BP_RockEnemy` _returnvalue_owneractor))
      (set `self.RockEnemy` _asbp_rock_enemy)))
  (return))

(fn `GetLineTrace`
  (returns (Actor :type "Actor Object Reference"))
  (bind _capsulecomponent (`Character.CapsuleComponent` (`self.RockEnemy`)))
  (bind _returnvalue (`SceneComponent.K2_GetComponentLocation` _capsulecomponent))
  (bind _outhit (`KismetSystemLibrary.LineTraceSingle` :`Start` _returnvalue :`End` (+ _returnvalue (* (`SceneComponent.GetForwardVector` _capsulecomponent) (`self.WeaponRange`))) :`TraceChannel` "TraceTypeQuery1" :`DrawDebugType` "Persistent"))
  (bind (_bblockinghit _binitialoverlap _time _distance _location _impactpoint _normal _impactnormal _physmat _hitactor) (`GameplayStatics.BreakHitResult` _outhit))
  (`/Engine/EditorBlueprintResources/StandardMacros.IsValid` _hitactor
    (:`Is Valid`
      (return _hitactor))))