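; GA_DoomAbility is a Gameplay Ability for firing weapons, with empty ShootWeapon and Reset hooks that appear intended for child overrides.
; Activation commits the ability, starts listening for the weapon event tag, calls ShootWeapon, then waits out the remaining cooldown before ending.
; ApplyEffect sends target data as a gameplay event, which the listener turns into the weapon's GameplayEffect.
; Ending stops both tasks, calling Reset if the delay task is valid.
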(event `self.K2_ActivateAbility`
  ;[1 1 1] Activate
  (`self.K2_CommitAbility`)
  (`self.WaitForEvent`)
  (`self.ShootWeapon`)
  ;[1 1 1] Ability duration
  (bind _asynctaskproxy (`GameplayTask_WaitDelay.TaskWaitDelay` null (`self.GetCooldownTimeRemaining`))
    (:`then`
      (set `self.shootRateDelayTask` _asynctaskproxy))
    (:`OnFinish`
      (`self.K2_EndAbility`))))

(event `WaitForEvent`
  ;[1 1 1] Wait for gameplay tag
  (bind (_asynctaskproxy _payload) (`AbilityTask_WaitGameplayEvent.WaitGameplayEvent` (`self.weaponEventTag`) null)
    (:`then`
      (set `self.gameplayEventWaitTask` _asynctaskproxy))
    (:`EventReceived`
      (`self.BP_ApplyGameplayEffectToTarget` (`.TargetData` (break `GameplayEventData` _payload)) (`self.weaponEffect`)))))

(event `ShootWeapon`)

(event `self.K2_OnEndAbility`
  (params (bWasCancelled :type Boolean))
  (bind _gameplayeventwaittask (`self.gameplayEventWaitTask`))
  (bind _shootratedelaytask (`self.shootRateDelayTask`))
  ;[1 1 1] Ability cleanup
  (`/Engine/EditorBlueprintResources/StandardMacros.IsValid` _gameplayeventwaittask
    (:`Is Valid`
      (`GameplayTask.EndTask` _gameplayeventwaittask))
    (:`Is Not Valid`
      _))
  (`/Engine/EditorBlueprintResources/StandardMacros.IsValid` _shootratedelaytask
    (:`Is Valid`
      (`GameplayTask.EndTask` _shootratedelaytask)
      (`self.Reset`))))

(fn `ApplyEffect`
  (params (AttackingActor :type "Actor Object Reference") (Target :type "Actor Object Reference"))
  (`AbilitySystemBlueprintLibrary.SendGameplayEventToActor` AttackingActor (`self.weaponEventTag`) (make `GameplayEventData` (struct) null Target null null (struct) (struct) (struct) 0.0 (`AbilitySystemBlueprintLibrary.AbilityTargetDataFromActor` Target))))

(fn `Reset`)