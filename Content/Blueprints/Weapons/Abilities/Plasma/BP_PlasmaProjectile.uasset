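; BP_PlasmaProjectile is a plasma projectile that damages enemies it overlaps.
; Each tick it billboards its Paper sprite on yaw only, turning it toward the player camera.
; On sphere overlap it skips the first-person character and applies GE_PlasmaDamage to BP_Enemy actors through the Gameplay Ability System.
; The enemy's own ability system component is both effect source and target, and the graph never destroys the projectile.
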(event `self.ReceiveTick`
  (params (DeltaSeconds :type "Float (single-precision)"))
  (bind _papersprite (`self.PaperSprite`))
  (bind (_returnvalue_roll _returnvalue_pitch _returnvalue_yaw) (`KismetMathLibrary.BreakRotator` (`KismetMathLibrary.FindLookAtRotation` (`SceneComponent.K2_GetComponentLocation` _papersprite) (`PlayerCameraManager.GetCameraLocation` (`GameplayStatics.GetPlayerCameraManager` 0)))))
  (`SceneComponent.K2_SetWorldRotation` _papersprite (`KismetMathLibrary.MakeRotator` 0.0 0.0 (- _returnvalue_yaw 90.0)) false false))

(event `self.Sphere.OnComponentBeginOverlap`
  (params (OverlappedComponent :type "PrimitiveComponent Object Reference") (OtherActor :type "Actor Object Reference") (OtherComp :type "PrimitiveComponent Object Reference") (OtherBodyIndex :type Integer) (bFromSweep :type Boolean) (SweepResult :type "HitResult Structure (by ref)"))
  (if (not (== (`GameplayStatics.GetObjectClass` OtherActor) "/Game/FirstPerson/Blueprints/BP_FirstPersonCharacter.BP_FirstPersonCharacter_C"))
    (bind _asbp_enemy (cast `/Game/Blueprints/Enemies/BP_Enemy` OtherActor))
    (bind _returnvalue (`AbilitySystemBlueprintLibrary.GetAbilitySystemComponent` _asbp_enemy))
    (`AbilitySystemComponent.BP_ApplyGameplayEffectToTarget` _returnvalue "/Game/Blueprints/Weapons/Abilities/Plasma/GE_PlasmaDamage.GE_PlasmaDamage_C" _returnvalue 0.0 (`AbilitySystemComponent.MakeEffectContext` _returnvalue))))

(fn `UserConstructionScript`)