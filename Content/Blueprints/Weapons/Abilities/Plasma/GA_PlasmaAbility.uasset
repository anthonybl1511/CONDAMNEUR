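; Gameplay ability that fires the player's plasma weapon.
; ShootWeapon requires a positive ability-system attribute, then applies the plasma spend effect to the owner and calls ShootPlasma on the BP_Plasma weapon.
; Helper functions lazily cache the first-person character and its child-actor weapon.
; GetLineTrace returns the actor hit along the camera's forward vector within weapon range, but the shooting path here never calls it.
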(event `self.ShootWeapon`
  (bind _playerplasmaweapon (`self.PlayerPlasmaWeapon`))
  ;[1 1 1] Shooting
  (`self.GetPlayer`)
  (if (> (`.ReturnValue` (`AbilitySystemBlueprintLibrary.GetFloatAttributeFromAbilitySystemComponent` (`FirstPersonCharacter.AbilitySystemComponent` (`self.Player`)) (struct :`AttributeName` "Plasma" :`Attribute` "/Script/CONDAMNEUR.FirstPersonAttributeSet:Plasma" :`AttributeOwner` "/Script/CoreUObject.Class'\"/Script/CONDAMNEUR.FirstPersonAttributeSet\"'"))) 0.0)
    (`self.GetWeapon`)
    (`/Engine/EditorBlueprintResources/StandardMacros.IsValid` _playerplasmaweapon
      (:`Is Valid`
        (`self.BP_ApplyGameplayEffectToOwner` "/Game/Blueprints/Weapons/Abilities/Plasma/GE_PlayerPlasmaSpend.GE_PlayerPlasmaSpend_C")
        (`/Game/Blueprints/Weapons/Arms/BP_Plasma.Shoot Plasma` _playerplasmaweapon)))))

(fn `GetLineTrace`
  (returns (Actor :type "Actor Object Reference"))
  (bind _firstpersoncamera (`/Game/FirstPerson/Blueprints/BP_FirstPersonCharacter.FirstPersonCamera` (`self.Player`)))
  (bind _returnvalue (`SceneComponent.K2_GetComponentLocation` _firstpersoncamera))
  (bind _outhit (`KismetSystemLibrary.LineTraceSingle` _returnvalue (+ _returnvalue (* (`SceneComponent.GetForwardVector` _firstpersoncamera) (`self.WeaponRange`))) "TraceTypeQuery1"))
  (bind (_bblockinghit _binitialoverlap _time _distance _location _impactpoint _normal _impactnormal _physmat _hitactor) (`GameplayStatics.BreakHitResult` _outhit))
  (`/Engine/EditorBlueprintResources/StandardMacros.IsValid` _hitactor
    (:`Is Valid`
      (return _hitactor))))

(fn `GetPlayer`
  (bind _returnvalue_owneractor (break `GameplayAbilityActorInfo` (`self.GetActorInfo`)))
  (`/Engine/EditorBlueprintResources/StandardMacros.IsValid` (`self.Player`)
    (:`Is Valid`
      _)
    (:`Is Not Valid`
      (bind _asbp_first_person_character (cast `/Game/FirstPerson/Blueprints/BP_FirstPersonCharacter` _returnvalue_owneractor))
      (set `self.Player` _asbp_first_person_character)))
  (return))

(fn `GetWeapon`
  (`/Engine/EditorBlueprintResources/StandardMacros.IsValid` (`self.PlayerPlasmaWeapon`)
    (:`Is Valid`
      _)
    (:`Is Not Valid`
      (bind _asbp_plasma (cast `/Game/Blueprints/Weapons/Arms/BP_Plasma` (`ChildActorComponent.ChildActor` (`/Game/FirstPerson/Blueprints/BP_FirstPersonCharacter.WeaponActor` (`self.Player`)))))
      (set `self.PlayerPlasmaWeapon` _asbp_plasma)))
  (return))