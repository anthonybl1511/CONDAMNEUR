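; Gameplay ability that fires the player's pistol and applies an effect to the character it hits.
; ShootWeapon lazily caches the owning first-person character and its child-actor pistol, then calls Shoot on the pistol.
; A Visibility line trace starts at the camera, but its end is forward times WeaponRange without adding the start location.
; A hit BP_FirstPersonCharacter becomes the ApplyEffect target, with the player as attacker.
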(event `self.ShootWeapon`
  (bind _playerpistolweapon (`self.PlayerPistolWeapon`))
  ;[1 1 1] Shooting
  (`self.GetPlayer`)
  (`self.GetWeapon`)
  (`/Engine/EditorBlueprintResources/StandardMacros.IsValid` _playerpistolweapon
    (:`Is Valid`
      (`/Game/Blueprints/Weapons/Arms/BP_Pistol.Shoot` _playerpistolweapon)
      (bind _actor (`self.GetLineTrace`))
      (bind _asbp_first_person_character (cast `/Game/FirstPerson/Blueprints/BP_FirstPersonCharacter` _actor))
      (`self.ApplyEffect` (`self.Player`) _asbp_first_person_character))))

(fn `GetLineTrace`
  (returns (Actor :type "Actor Object Reference"))
  (bind _firstpersoncamera (`/Game/FirstPerson/Blueprints/BP_FirstPersonCharacter.FirstPersonCamera` (`self.Player`)))
  (bind _outhit (`KismetSystemLibrary.LineTraceSingle` (`SceneComponent.K2_GetComponentLocation` _firstpersoncamera) (* (`KismetMathLibrary.GetForwardVector` (`SceneComponent.K2_GetComponentRotation` _firstpersoncamera)) (`self.WeaponRange`)) "TraceTypeQuery1"))
  (bind (_bblockinghit _binitialoverlap _time _distance _location _impactpoint _normal _impactnormal _physmat _hitactor) (`GameplayStatics.BreakHitResult` _outhit))
  (`/Engine/EditorBlueprintResources/StandardMacros.IsValid` _hitactor
    (:`Is Valid`
      (return _hitactor))))

(fn `GetPlayer`
  (bind _returnvalue_owneractor (break `GameplayAbilityActorInfo` (`self.GetActorInfo`)))
  (`/Engine/EditorBlueprintResources/StandardMacros.IsValid` (`self.Player`)
    (:`Is Valid`
      _)
    (:`Is Not Valid`
      (bind _asbp_first_person_character (cast `/Game/FirstPerson/Blueprints/BP_FirstPersonCharacter` _returnvalue_owneractor))
      (set `self.Player` _asbp_first_person_character)))
  (return))

(fn `GetWeapon`
  (`/Engine/EditorBlueprintResources/StandardMacros.IsValid` (`self.PlayerPistolWeapon`)
    (:`Is Valid`
      _)
    (:`Is Not Valid`
      (bind _asbp_pistol (cast `/Game/Blueprints/Weapons/Arms/BP_Pistol` (`ChildActorComponent.ChildActor` (`/Game/FirstPerson/Blueprints/BP_FirstPersonCharacter.WeaponActor` (`self.Player`)))))
      (set `self.PlayerPistolWeapon` _asbp_pistol)))
  (return))