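; BP_WeaponPickup is a world pickup that grants a weapon to the player on touch.
; An overlapping BP_FirstPersonCharacter is told to equip the pickup's WeaponType, then the pickup destroys itself.
; Each tick, WeaponSprite rotates on yaw only to face the player camera, billboarding the 2D sprite while keeping it upright.
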(event `self.ReceiveActorBeginOverlap`
  (params (OtherActor :type "Actor Object Reference"))
  (bind _asbp_first_person_character (cast `/Game/FirstPerson/Blueprints/BP_FirstPersonCharacter` OtherActor))
  (`/Game/FirstPerson/Blueprints/BP_FirstPersonCharacter.EquipWeapon` _asbp_first_person_character (`self.Weapon type`))
  (`self.K2_DestroyActor`))

(event `self.ReceiveTick`
  (params (DeltaSeconds :type "Float (single-precision)"))
  (bind _weapon_sprite (`self.Weapon Sprite`))
  (bind (_returnvalue_roll _returnvalue_pitch _returnvalue_yaw) (`KismetMathLibrary.BreakRotator` (`KismetMathLibrary.FindLookAtRotation` (`SceneComponent.K2_GetComponentLocation` _weapon_sprite) (`PlayerCameraManager.GetCameraLocation` (`GameplayStatics.GetPlayerCameraManager` 0)))))
  (`SceneComponent.K2_SetWorldRotation` _weapon_sprite (`KismetMathLibrary.MakeRotator` 0.0 0.0 (- _returnvalue_yaw 90.0)) false false))

(fn `UserConstructionScript`)