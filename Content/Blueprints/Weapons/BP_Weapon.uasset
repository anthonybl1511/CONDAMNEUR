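; BP_Weapon is a hitscan weapon with empty FireWeapon and StopFire events and a reusable Shoot function.
; Shoot line-traces forward from the Raycast component out to RaycastDistance, against static, dynamic and pawn objects, ignoring itself and the player character.
; On a hit it applies WeaponDamage to the actor struck.
; The trace leaves debug drawing on for a set duration, and nothing in this file calls Shoot.
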(event `FireWeapon`)

(event `StopFire`)

(fn `Shoot`
  (bind _returnvalue (`SceneComponent.K2_GetComponentLocation` (`self.Raycast`)))
  (bind (_outhit _returnvalue_2) (`KismetSystemLibrary.LineTraceSingleForObjects` _returnvalue (+ _returnvalue (* (`KismetMathLibrary.GetForwardVector` (`SceneComponent.K2_GetComponentRotation` (`self.Raycast`))) (`self.raycastDistance`))) (`|MakeArray` "ObjectTypeQuery1" "ObjectTypeQuery2" "ObjectTypeQuery3" :!type "EObjectTypeQuery Enum") false (`|MakeArray` self (`GameplayStatics.GetPlayerCharacter` 0) :!type "Actor Object Reference") "ForDuration"))
  (if _returnvalue_2
    (`GameplayStatics.ApplyDamage` (`.HitActor` (`GameplayStatics.BreakHitResult` _outhit)) (`self.weaponDamage`))))

(fn `UserConstructionScript`)