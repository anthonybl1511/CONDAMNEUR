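; BP_StatPickup is an item pickup for health or armor, in small or large size, shown as a flipbook sprite.
; The construction script sets the flipbook, sprite scale and gameplay tag from the pickup's type and size.
; Two check functions read a Gameplay Ability System attribute and add or remove Full health or armor tags on the pickup's tag, comparing against hardcoded maximums.
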(fn `FullArmorCheck`
  (params (AbilitySystem :type "AbilitySystemComponent Object Reference"))
  (bind _pickuptag (`self.PickupTag`))
  (if (== (`.ReturnValue` (`AbilitySystemBlueprintLibrary.GetFloatAttributeFromAbilitySystemComponent` AbilitySystem (struct :`AttributeName` "Armor" :`Attribute` "/Script/CONDAMNEUR.FirstPersonAttributeSet:Armor" :`AttributeOwner` "/Script/CoreUObject.Class'\"/Script/CONDAMNEUR.FirstPersonAttributeSet\"'"))) 40.0)
    (`BlueprintGameplayTagLibrary.AddGameplayTag` _pickuptag (struct :`TagName` "Player.Armor.Full"))
    (else
      (`BlueprintGameplayTagLibrary.RemoveGameplayTag` _pickuptag (struct :`TagName` "Player.Armor.Full")))))

(fn `FullHealthCheck`
  (params (AbilitySystem :type "AbilitySystemComponent Object Reference"))
  (bind _pickuptag (`self.PickupTag`))
  (if (== (`.ReturnValue` (`AbilitySystemBlueprintLibrary.GetFloatAttributeFromAbilitySystemComponent` AbilitySystem (struct :`AttributeName` "Health" :`Attribute` "/Script/CONDAMNEUR.FirstPersonAttributeSet:Health" :`AttributeOwner` "/Script/CoreUObject.Class'\"/Script/CONDAMNEUR.FirstPersonAttributeSet\"'"))) 100.0)
    (`BlueprintGameplayTagLibrary.AddGameplayTag` _pickuptag (struct :`TagName` "Player.Health.Full"))
    (else
      (`BlueprintGameplayTagLibrary.RemoveGameplayTag` _pickuptag (struct :`TagName` "Player.Health.Full")))))

(fn `SetStatPickupFlipbook`
  (bind _itemsprite (`self.ItemSprite`))
  (bind _itemsprite_2 (`self.ItemSprite`))
  (switch `/Game/Blueprints/ENUMs/ENUM_PickupType` (`self.PickupType`)
    (:`NewEnumerator0`
      (`PaperFlipbookComponent.SetFlipbook` _itemsprite "/Game/Sprites/UI/Damage_Icons2.Damage_Icons2")
      (switch `/Game/Blueprints/ENUMs/ENUM_PickupSize` (`self.PickupSize`)
        (:`NewEnumerator0`
          (`SceneComponent.SetRelativeScale3D` _itemsprite_2 (1.0 1.0 1.0))
          (set `self.PickupTag` (struct :`GameplayTags` (struct :`(TagName` "Pickup.Armor.Small")))))
        (:`NewEnumerator1`
          (`SceneComponent.SetRelativeScale3D` _itemsprite_2 (2.0 2.0 2.0))
          (set `self.PickupTag` (struct :`GameplayTags` (struct :`(TagName` "Pickup.Armor.Large")))))))
    (:`NewEnumerator1`
      (`PaperFlipbookComponent.SetFlipbook` _itemsprite "/Game/Sprites/UI/Damage_Icons1.Damage_Icons1")
      (switch `/Game/Blueprints/ENUMs/ENUM_PickupSize` (`self.PickupSize`)
        (:`NewEnumerator0`
          (`SceneComponent.SetRelativeScale3D` _itemsprite_2 (1.0 1.0 1.0))
          (set `self.PickupTag` (struct :`GameplayTags` (struct :`(TagName` "Pickup.Health.Small")))))
        (:`NewEnumerator1`
          (`SceneComponent.SetRelativeScale3D` _itemsprite_2 (2.0 2.0 2.0))
          (set `self.PickupTag` (struct :`GameplayTags` (struct :`(TagName` "Pickup.Health.Large")))))))))

(fn `UserConstructionScript`
  (`parent.UserConstructionScript`)
  (`self.SetStatPickupFlipbook`))