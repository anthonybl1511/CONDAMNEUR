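; Weapon pickup actor that grants a weapon to the first-person player character on overlap.
; The construction script sets the item sprite's flipbook from the WeaponType variable, covering pistol and plasma gun, with no flipbook for None.
; When BP_FirstPersonCharacter overlaps it, the actor passes WeaponType to PickupWeapon and destroys itself.
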(event `self.ReceiveActorBeginOverlap`
  (params (OtherActor :type "Actor Object Reference"))
  (bind _asbp_first_person_character (cast `/Game/FirstPerson/Blueprints/BP_FirstPersonCharacter` OtherActor))
  (`/Game/FirstPerson/Blueprints/BP_FirstPersonCharacter.PickupWeapon` _asbp_first_person_character (`self.Weapon type`))
  (`self.K2_DestroyActor`))

(fn `UserConstructionScript`
  (bind _itemsprite (`self.ItemSprite`))
  (switch `/Game/Blueprints/ENUMs/ENUM_WeaponList` (`self.Weapon type`)
    (:`NewEnumerator0`
      (`PaperFlipbookComponent.SetFlipbook` _itemsprite null))
    (:`NewEnumerator1`
      (`PaperFlipbookComponent.SetFlipbook` _itemsprite "/Game/Sprites/Weapons/Pistol/PistolPickup_Flipbook.PistolPickup_Flipbook"))
    (:`NewEnumerator2`
      (`PaperFlipbookComponent.SetFlipbook` _itemsprite "/Game/Sprites/Weapons/PlasmaGun/FB_Plasma_Pickup.FB_Plasma_Pickup"))))